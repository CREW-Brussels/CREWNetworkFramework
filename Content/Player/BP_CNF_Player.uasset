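; BP_CNF_Player is the player Blueprint that links its PlayerState to a group in the CNF game mode.
; On BeginPlay, a locally controlled player passes the game mode's GroupIndex to its PlayerState, and on EndPlay the server removes that state from its Group.
; While locally viewed, it calls Apply on the PlayerState every Tick.
; ViewLocally only checks local viewing and performs no action.
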(event EventBeginPlay
  (|CallParentFunction)
  (if (Pawn|IsLocallyControlled)
    (bind _asbp_cnf_mode (Utilities|Casting|CastToBP_CNF_Mode (Game|GetGameMode)))
    (bind _asbp_cnf_player_state (Utilities|Casting|CastToBP_CNF_PlayerState (Variables|GetPlayerState)))
    (Default|SetGroupIndex _asbp_cnf_player_state (Variables|/CREWNetworkFramework/Mode/BP_CNF_Mode.BP_CNF_Mode_C|GetGroupIndex _asbp_cnf_mode))))

(event EventTick
  (params (DeltaSeconds :type Float%20%28single-precision%29))
  (|CallParentFunction DeltaSeconds)
  (if (Pawn|IsLocallyViewed)
    (bind _asbp_cnf_player_state (Utilities|Casting|CastToBP_CNF_PlayerState (Variables|GetPlayerState)))
    (Default|Apply _asbp_cnf_player_state)))

(event EventEndPlay
  (params (EndPlayReason :type EEndPlayReason%20Enum :default "Destroyed"))
  (|CallParentFunction EndPlayReason)
  (if (Networking|IsServer)
    (bind _asbp_cnf_player_state (Utilities|Casting|CastToBP_CNF_PlayerState (Variables|GetPlayerState)))
    (Default|RemovePlayer (Variables|/CREWNetworkFramework/State/BP_CNF_PlayerState.BP_CNF_PlayerState_C|GetGroup _asbp_cnf_player_state) _asbp_cnf_player_state)))

(fn ConstructionScript
  (|CallParentFunction))

(fn ViewLocally
  (if (Pawn|IsLocallyViewed)
    _))