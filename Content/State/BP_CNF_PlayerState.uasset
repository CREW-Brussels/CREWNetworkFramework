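; BP_CNF_PlayerState is the CNF player state, holding a per-player context object and handling group membership.
; On BeginPlay it constructs and stores a BP_CNF_Context.
; SetGroupIndex casts to BP_CNF_GameState and adds this player state to the group at the given index.
; ChangeVisibility only stores a CubeVisible flag that nothing here reads, and Apply is an empty stub.
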(event Custom|SetGroupIndex
  (params (Group :type Integer))
  (bind _asbp_cnf_game_state (Utilities|Casting|CastToBP_CNF_GameState (Game|GetGameState)))
  (Default|AddPlayer (Utilities|Array|Get(acopy) (Variables|/CREWNetworkFramework/State/BP_CNF_GameState.BP_CNF_GameState_C|GetGroups _asbp_cnf_game_state) Group) self))

(event Custom|ChangeVisibility
  (params (NewParam :type Boolean))
  (Variables|Default|SetCubeVisible NewParam))

(event EventBeginPlay
  (|CallParentFunction)
  (bind _returnvalue (Game|ConstructObjectfromClass "/CREWNetworkFramework/Context/BP_CNF_Context.BP_CNF_Context_C"))
  (Variables|Default|SetContext _returnvalue))

(event EventTick
  (params (DeltaSeconds :type Float%20%28single-precision%29))
  (|CallParentFunction DeltaSeconds) ; This node is disabled and will not be called.\nDrag off pins to build functionality.
)

(fn ConstructionScript
  (|CallParentFunction))

(fn Apply)