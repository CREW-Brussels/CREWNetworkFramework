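; BP_CNF_Trigger is a server-only trigger actor that destroys itself on clients at BeginPlay.
; Its Enter and Leave functions call Start and Stop on each entry in its Actions array, passing along the player state.
; With OnlyOnce set, it records itself in a context's TriggerEntered and TriggerLeft lists to avoid repeats.
; The Context enum scopes that record to the player, their group or the game state.
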(event EventBeginPlay
  (if (not (Networking|IsServer))
    (Actor|DestroyActor)))

(event EventTick
  (params (DeltaSeconds :type Float%20%28single-precision%29)))

(fn ConstructionScript)

(fn Enter
  (params (State :type BP%20CNF%20Player%20State%20Object%20Reference))
  (bind _self self)
  (if (Networking|IsServer)
    (if (Variables|Default|GetOnly%20Once)
      (bind _contextout (CallFunction|GetContext State))
      (if (not (Utilities|Set|Contains (Variables|/CREWNetworkFramework/Context/BP_CNF_Context.BP_CNF_Context_C|GetTriggerEntered _contextout) _self))
        (Utilities|Set|Add (Variables|/CREWNetworkFramework/Context/BP_CNF_Context.BP_CNF_Context_C|GetTriggerEntered _contextout) _self)
        (for _array_element (Variables|Default|GetActions) :!label _label
          (Default|Start _array_element State)))
      (else
        (goto _label)))))

(fn Leave
  (params (State :type BP%20CNF%20Player%20State%20Object%20Reference))
  (bind _self self)
  (if (Networking|IsServer)
    (if (Variables|Default|GetOnly%20Once)
      (bind _contextout (CallFunction|GetContext State))
      (if (not (Utilities|Set|Contains (Variables|/CREWNetworkFramework/Context/BP_CNF_Context.BP_CNF_Context_C|GetTriggerLeft _contextout) _self))
        (Utilities|Set|Add (Variables|/CREWNetworkFramework/Context/BP_CNF_Context.BP_CNF_Context_C|GetTriggerLeft _contextout) _self)
        (for _array_element (Variables|Default|GetActions) :!label _label
          (Default|Stop _array_element State)))
      (else
        (goto _label)))))

(fn GetContext
  (params (Player :type BP%20CNF%20Player%20State%20Object%20Reference))
  (switch Utilities|FlowControl|Switch|Switchon (Variables|Default|GetContext)
    (:NewEnumerator0
      (return (Variables|/CREWNetworkFramework/State/BP_CNF_PlayerState.BP_CNF_PlayerState_C|GetContext Player)))
    (:NewEnumerator1
      (return (Variables|/CREWNetworkFramework/State/BP_CNF_GroupState.BP_CNF_GroupState_C|GetContext (Variables|/CREWNetworkFramework/State/BP_CNF_PlayerState.BP_CNF_PlayerState_C|GetGroup Player))))
    (:NewEnumerator2
      (bind _asbp_cnf_game_state (Utilities|Casting|CastToBP_CNF_GameState (Game|GetGameState)))
      (return (Variables|/CREWNetworkFramework/State/BP_CNF_GameState.BP_CNF_GameState_C|GetContext _asbp_cnf_game_state)))))